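; House door that flags when the player is in range and runs the day change through its NewDay event.
; NewDay disables input, plays a fade sequence and spawns each person door's next queued mission where the current one is missing or ended.
; It then advances the day count, fails missions past their deadline and re-enables all Interactibles.
; Player input returns after a short delay.
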(event Custom|NewDay
  (Input|DisableInput (Game|GetPlayerCharacter 0) (Game|GetPlayerController 0))
  (bind _returnvalue (Sequencer|Player|CreateLevelSequencePlayer "/Game/Cinematics/NewDayFade.NewDayFade"))
  (Sequencer|Player|Play _returnvalue :!class /Script/MovieScene.MovieSceneSequencePlayer)
  (for _array_element (Variables|Default|GetAllPersonDoors)
    (if (Utilities|IsValid (Variables|/Game/Blueprints/PersonDoor.PersonDoor_C|GetMissionOnGoing _array_element))
      (if (Variables|/Game/Blueprints/Missions/MissionBase.MissionBase_C|GetMissionEnded (Actor|GetComponentbyClass (Variables|/Game/Blueprints/PersonDoor.PersonDoor_C|GetMissionOnGoing _array_element) "/Game/Blueprints/Missions/MissionBase.MissionBase_C"))
        (bind _returnvalue_2 (Game|SpawnActorfromClass (Utilities|Array|Get(acopy) (Variables|/Game/Blueprints/PersonDoor.PersonDoor_C|GetMissions _array_element)) (Transformation|GetActorTransform) "Undefined" "MultiplyWithRoot" 0 0 :!label _label))
        (Variables|/Game/Blueprints/PersonDoor.PersonDoor_C|SetMissionOnGoing _array_element _returnvalue_2)
        (Utilities|Array|RemoveIndex (Variables|/Game/Blueprints/PersonDoor.PersonDoor_C|GetMissions _array_element))
        (Utilities|FlowControl|Delay 1.15)
        (Input|EnableInput (Game|GetPlayerCharacter 0) (Game|GetPlayerController 0)))
      (else
        (goto _label))))
  (Math|Integer|IncrementInt (Variables|Default|GetDaysPassed)
    (:%20%20
      (for _array_element_2 (Variables|Default|GetAllPersonDoors)
        (bind _asactor (Utilities|Casting|CastToActor (Variables|/Game/Blueprints/PersonDoor.PersonDoor_C|GetMissionOnGoing _array_element_2)))
        (if (not (< (- (Variables|Default|GetDaysPassed) (Variables|/Game/Blueprints/Missions/MissionBase.MissionBase_C|GetDayStarted (Utilities|Array|Get(acopy) (Actor|GetComponentsByClass _asactor "/Game/Blueprints/Missions/MissionBase.MissionBase_C")))) (Variables|/Game/Blueprints/Missions/MissionBase.MissionBase_C|GetDaysToComplete (Utilities|Array|Get(acopy) (Actor|GetComponentsByClass _asactor "/Game/Blueprints/Missions/MissionBase.MissionBase_C")))))
          (Variables|/Game/Blueprints/Missions/MissionBase.MissionBase_C|SetMissionEnded (Utilities|Array|Get(acopy) (Actor|GetComponentsByClass _asactor "/Game/Blueprints/Missions/MissionBase.MissionBase_C")) true)
          (Default|MissionFailed (Utilities|Array|Get(acopy) (Actor|GetComponentsByClass _asactor "/Game/Blueprints/Missions/MissionBase.MissionBase_C")))))
      (bind _outactors (Actor|GetAllActorsOfClass "/Game/Blueprints/Interactible.Interactible_C"))
      (for _array_element_3 _outactors
        (bind _asinteractible (Utilities|Casting|CastToInteractible _array_element_3))
        (Variables|/Game/Blueprints/Interactible.Interactible_C|SetCanInteract _asinteractible true))
      (Utilities|FlowControl|Delay 1.15)
      (Input|EnableInput (Game|GetPlayerCharacter 0) (Game|GetPlayerController 0)))))

(event Collision|EventActorBeginOverlap
  (params (OtherActor :type Actor%20Object%20Reference))
  (if (== OtherActor (Game|GetPlayerCharacter 0))
    (Variables|Default|SetCanBeInteracted true)))

(event Collision|EventActorEndOverlap
  (params (OtherActor :type Actor%20Object%20Reference))
  (if (== OtherActor (Game|GetPlayerCharacter 0))
    (Variables|Default|SetCanBeInteracted false)))

(fn ConstructionScript)