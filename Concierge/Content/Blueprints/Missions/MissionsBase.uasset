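; MissionsBase is a base Blueprint for missions that prints temporary intro text on BeginPlay.
; Its Mission function, when interactibles are needed, spawns the InteractibleInstance class at every spawn point or at one random point, depending on a multiple-interactibles flag.
; Each spawned actor is stored in MissionTarget, and MissionEnd is an empty stub.
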(event EventBeginPlay
  (Development|PrintString (Variables|Default|GetTemp_IntroText)))

(fn ConstructionScript)

(fn Mission
  (if (Variables|Default|GetNeedToSpawnInteractible%20)
    (if (Variables|Default|GetMultipleInteractbles)
      (for _array_element (Variables|Default|GetSpawnPoints)
        (bind _returnvalue (Game|SpawnActorfromClass (Variables|Default|GetInteractibleInstance) _array_element "Undefined" "MultiplyWithRoot" 0 0))
        (Utilities|Array|Add (Variables|Default|GetMissionTarget) _returnvalue))
      (else
        (bind _returnvalue_2 (Game|SpawnActorfromClass (Variables|Default|GetInteractibleInstance) (.OutItem (Utilities|Array|Random (Variables|Default|GetSpawnPoints))) "Undefined" "MultiplyWithRoot" 0 0))
        (Utilities|Array|Add (Variables|Default|GetMissionTarget) _returnvalue_2)))))

(fn MissionEnd)