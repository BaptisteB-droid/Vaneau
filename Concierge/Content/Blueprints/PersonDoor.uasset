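; PersonDoor is an actor that plays mission dialog when the player walks into it while a mission is ongoing.
; On overlap with the player character, it finds the MissionBase component on MissionOnGoing and calls PlayDialog with itself.
; If that mission has ended, it waits ten seconds, prints a goodbye, then destroys the mission actor and clears the reference.
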(event Collision|EventActorBeginOverlap
  (params (OtherActor :type Actor%20Object%20Reference))
  (if (and (== OtherActor (Game|GetPlayerCharacter 0)) (Utilities|IsValid (Variables|Default|GetMissionOnGoing)))
    (bind _asmission_base (Utilities|Casting|CastToMissionBase (Actor|GetComponentbyClass (Variables|Default|GetMissionOnGoing) "/Game/Blueprints/Missions/MissionBase.MissionBase_C")))
    (Default|PlayDialog _asmission_base self)
    (if (Variables|/Game/Blueprints/Missions/MissionBase.MissionBase_C|GetMissionEnded (Actor|GetComponentbyClass (Variables|Default|GetMissionOnGoing) "/Game/Blueprints/Missions/MissionBase.MissionBase_C"))
      (Utilities|FlowControl|Delay 1e+01)
      (Development|PrintString "B-bye")
      (Actor|DestroyActor (Variables|Default|GetMissionOnGoing))
      (Variables|Default|SetMissionOnGoing 0))))

(fn ConstructionScript)