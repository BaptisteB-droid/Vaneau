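; Interactible is an actor that the player can interact with a counted number of times, with ties to a parent mission.
; Overlap events add it to and remove it from the InteractibleList on BP_FirstPersonCharacter.
; Interact decrements the remaining count, clears CanInteract and prints debug messages.
; When the count runs out and DestroyedOnEnd is set, it removes itself from MissionBase's InteractiblesSpawned list and destroys itself.
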(event Custom|Interact
  (Variables|Default|SetInteracted true)
  (Variables|Default|SetNumberOfInteractions (- (Variables|Default|GetNumberOfInteractions) 1))
  (Development|PrintString (Utilities|String|Append "Interacted with" (Utilities|GetObjectName self)))
  (Variables|Default|SetCanInteract false)
  (if (> (Variables|Default|GetNumberOfInteractions) 0)
    (Development|PrintString "Nothing Happes")
    (elif (Variables|Default|GetDestroyedOnEnd)
      (CallFunction|RemoveInteractible))))

(event Collision|EventActorBeginOverlap
  (params (OtherActor :type Actor%20Object%20Reference))
  (if (== OtherActor (Game|GetPlayerCharacter 0))
    (bind _asbp_first_person_character (Utilities|Casting|CastToBP_FirstPersonCharacter (Game|GetPlayerCharacter 0)))
    (Utilities|Array|Add (Variables|/Game/FirstPerson/Blueprints/BP_FirstPersonCharacter.BP_FirstPersonCharacter_C|GetInteractibleList _asbp_first_person_character) self)))

(event Collision|EventActorEndOverlap
  (params (OtherActor :type Actor%20Object%20Reference))
  (if (== OtherActor (Game|GetPlayerCharacter 0))
    (bind _asbp_first_person_character (Utilities|Casting|CastToBP_FirstPersonCharacter (Game|GetPlayerCharacter 0)))
    (Utilities|Array|RemoveItem (Variables|/Game/FirstPerson/Blueprints/BP_FirstPersonCharacter.BP_FirstPersonCharacter_C|GetInteractibleList _asbp_first_person_character) self)))

(fn ConstructionScript)

(fn RemoveInteractible
  (bind _asmission_base (Utilities|Casting|CastToMissionBase (Variables|Default|GetMissionParent)))
  (Utilities|Array|RemoveItem (Variables|/Game/Blueprints/Missions/MissionBase.MissionBase_C|GetInteractiblesSpawned _asmission_base) self)
  (Actor|DestroyActor))